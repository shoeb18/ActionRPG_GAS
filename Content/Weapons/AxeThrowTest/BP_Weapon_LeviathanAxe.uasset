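; Throwable, recallable axe weapon that flies along the camera forward, sticks into what it hits and plays a death animation on enemies.
; An AxeState enum drives Tick, spinning the mesh in flight.
; While recalling, location chases the player's hand socket, mixing VInterpTo on X/Z with a Timeline-driven lerp on Y.
; Sphere overlap handles impacts and the catch, which plays a montage, reattaches the axe and fires a GameplayCue.
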(event `self.ReceiveTick`
  (params (DeltaSeconds :type "Float (single-precision)"))
  (bind (_returnvalue_x _returnvalue_y _returnvalue_z) (`KismetMathLibrary.BreakVector` (`KismetMathLibrary.VInterpTo` (`self.K2_GetActorLocation`) (`self.TargetLocation`) DeltaSeconds 10.0)))
  (switch `/Game/Weapons/AxeThrowTest/E_AxeState` (`self.AxeState`)
    (:`NewEnumerator1`
      (`SceneComponent.K2_AddLocalRotation` (`self.WeaponMesh`) (`KismetMathLibrary.MakeRotator` (* (* DeltaSeconds (`self.RotationSpeed`)) -1.0)) false false :!label _label))
    (:`NewEnumerator3`
      (`|ExecutionSequence`
        (:`then_0`
          (goto _label))
        (:`then_1`
          (bind (_direction _recallalpha) (`Timeline|Timeline`)
            (:`Update`
              (bind _ascharacter (cast `Character` (`GameplayStatics.GetPlayerPawn` 0)))
              (bind _output_get (set `self.TargetLocation` (`SceneComponent.GetSocketLocation` (`Character.Mesh` _ascharacter) "AxeSocket"))))))
        (:`then_2`
          (bind (_returnvalue_x_2 _returnvalue_y_2) (`KismetMathLibrary.BreakVector` (`KismetMathLibrary.VLerp` _output_get (`self.K2_GetActorLocation`) _recallalpha)))
          (`self.K2_SetActorLocation` (`KismetMathLibrary.MakeVector` _returnvalue_x _returnvalue_y_2 _returnvalue_z))
          (bind _ascharacter_2 (cast `Character` (`GameplayStatics.GetPlayerPawn` 0)))
          (set `self.TargetLocation` (`SceneComponent.GetSocketLocation` (`Character.Mesh` _ascharacter_2) "AxeSocket")))))))

(event `self.Sphere.OnComponentBeginOverlap`
  (params (OverlappedComponent :type "PrimitiveComponent Object Reference") (OtherActor :type "Actor Object Reference") (OtherComp :type "PrimitiveComponent Object Reference") (OtherBodyIndex :type Integer) (bFromSweep :type Boolean) (SweepResult :type "HitResult Structure (by ref)"))
  (if (== OtherActor (`GameplayStatics.GetPlayerPawn` 0))
    (if (`|EnumEquality` (`self.AxeState`) "NewEnumerator3")
      (set `self.AxeState` "NewEnumerator4")
      (bind _ascharacter (cast `Character` (`GameplayStatics.GetPlayerPawn` 0)))
      (bind _mesh (`Character.Mesh` _ascharacter))
      (`|PlayMontage` _mesh "/Game/Weapons/AxeThrowTest/AxeRecallEnd.AxeRecallEnd"
        (:`then`
          (`self.K2_AttachToComponent` _mesh (`.EquippedSocketName_10_852FF28A4E1E50D52BF4CDAAAA14F530` (break `/Game/Weapons/Data/S_WeaponConfig` (`self.WeaponConfig`))) "SnapToTarget" "SnapToTarget" "SnapToTarget")
          (set `self.AxeState` "NewEnumerator0")
          (`SceneComponent.ResetRelativeTransform` (`self.WeaponMesh`))
          (`GameplayCueFunctionLibrary.ExecuteGameplayCueOnActor` (`GameplayStatics.GetPlayerPawn` 0) (struct :`TagName` "GameplayCue.Test") (`AbilitySystemBlueprintLibrary.MakeGameplayCueParameters` 0.0)))))
    (else
      (set `MovementComponent.Velocity` (0.0 0.0 0.0) (`self.ProjectileMovement`))
      (`self.K2_AttachToComponent` self OtherComp "None" "KeepWorld" "KeepWorld" "KeepWorld" true)
      (set `self.AxeState` "NewEnumerator2")
      (bind _asbp_enemy_base (cast `/Game/GAS/Characters/BP_Enemy_Base` OtherActor))
      (`SkeletalMeshComponent.PlayAnimation` (`Character.Mesh` _asbp_enemy_base) "/Game/Assets/Animations/AxeAndShield/Animations/InPlace/Death_IP.Death_IP" false))))

(event `Play Throw Montage`
  (params (InSkeletalMeshComponent :type "SkeletalMeshComponent Object Reference"))
  (`|PlayMontage` InSkeletalMeshComponent (`self.ThrowAnim`)))

(event `Play Recall Montage`
  (params (InSkeletalMeshComponent :type "SkeletalMeshComponent Object Reference"))
  (`|PlayMontage` InSkeletalMeshComponent "/Game/Weapons/AxeThrowTest/Recall_Loop_Montage.Recall_Loop_Montage" -1.0))

(fn `Recall`
  (params (InSkeletalMeshComponent :type "SkeletalMeshComponent Object Reference"))
  (`self.Play Recall Montage` InSkeletalMeshComponent)
  (`self.K2_DetachFromActor` "KeepWorld" "KeepWorld" "KeepWorld"))

(fn `ThrowAxe`
  (bind _sphere (`self.Sphere`))
  (if (`|EnumEquality` (`self.AxeState`) "NewEnumerator0")
    (set `self.AxeState` "NewEnumerator1")
    (`PrimitiveComponent.SetCollisionEnabled` _sphere "QueryAndPhysics")
    (`PrimitiveComponent.SetCollisionResponseToAllChannels` _sphere "ECR_Overlap")
    (`self.K2_DetachFromActor` "KeepWorld" "KeepWorld" "KeepWorld")
    (set `MovementComponent.Velocity` (* (`self.GetActorForwardVector` (`GameplayStatics.GetPlayerCameraManager` 0)) 2000.0) (`self.ProjectileMovement`))))

(fn `UserConstructionScript`
  (`parent.UserConstructionScript`))